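; BP_Pawn is the main player pawn, acting as a free-moving camera with zoom.
; Forward, Right and Zoom axis inputs update a desired world-space location and a clamped desired spring arm length.
; Tick smoothly interpolates the actor position and arm length toward those targets.
; Movement follows world X and Y without sweep, and input steps are not scaled by delta time.
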(event EventTick
  (params (DeltaSeconds :type Float%20%28single-precision%29))
  (bind _springarm (Variables|Default|GetSpringArm))
  ;[1 1 1] CAMERA
  ;;[1 1 1] TICK: EVENTO CHE VIENE CHIAMATO AD OGNI FRAME
  (Variables|/Script/Engine.SpringArmComponent|SetTargetArmLength _springarm (Math|Interpolation|FInterpTo (Variables|/Script/Engine.SpringArmComponent|GetTargetArmLength _springarm) (Variables|Default|GetZoom_Desired) DeltaSeconds 2.0))
  (Transformation|SetActorLocation (Math|Interpolation|VInterpTo (Transformation|GetActorLocation) (Variables|Default|GetLocation_Desired) DeltaSeconds 5.0) false false))

(event EventBeginPlay
  ;[1 1 1] THE FIRST FRAME
  (Variables|Default|SetLocation_Desired (Transformation|GetActorLocation)))

(event Input|AxisEvents|InputAxisInputAxis_Zoom
  (params (AxisValue :type Float%20%28single-precision%29))
  ;[1 1 1] ZOOM
  ;;[1 1 1] Blocco "Promote to variable". Variabile modificata in "Zoom Desired"
  (Variables|Default|SetZoom_Desired (Math|Float|Clamp(Float) (+ (Variables|Default|GetZoom_Desired) (* AxisValue 4e+01)) 1e+02 5e+03)))

(event Input|AxisEvents|InputAxisInputAxis_Right
  (params (AxisValue :type Float%20%28single-precision%29))
  ;[1 1 1] set Location Desired
  (Variables|Default|SetLocation_Desired (+ (Variables|Default|GetLocation_Desired) (Math|Vector|MakeVector 0.0 (* AxisValue 4e+01) 0.0))))

(event Input|AxisEvents|InputAxisInputAxis_Forward
  (params (AxisValue :type Float%20%28single-precision%29))
  ;[1 1 1] set Location Desired
  (Variables|Default|SetLocation_Desired (+ (Variables|Default|GetLocation_Desired) (Math|Vector|MakeVector (* AxisValue 4e+01) 0.0 0.0))))

(fn ConstructionScript)